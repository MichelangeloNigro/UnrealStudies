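; MeteorBP is a boss-related meteor actor that plays its audio on spawn and reports landing on soil to its spawner.
; BeginPlay binds a hit handler that, while a boolean guard is set, checks the hit actor for the "soil" tag, sets the spawner's MeteorOnSoil flag and clears the guard.
; The handler then gathers all meteors, but the loop that would unbind and disarm them is disconnected.
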(event Custom|OnActorHit_Event_0
  (params (SelfActor :type Actor%20Object%20Reference) (OtherActor :type Actor%20Object%20Reference) (NormalImpulse :type Vector) (Hit :type Hit%20Result%20Structure%20%28by%20ref%29))
  (if (Variables|Default|GetNewVar_0)
    (if (Actor|ActorHasTag (.hitactor Hit) "soil")
      (Variables|/Script/UnrealStudies.Boss|SetMeteorOnSoil (Class|RealMeteor|GetSpawner) true)
      (Variables|Default|SetNewVar_0 false)
      (bind _outactors (Actor|GetAllActorsOfClass "MeteorBP_C")))))

(event EventBeginPlay
  (Collision|AssignOnActorHit (delegate Custom|OnActorHit_Event_0))
  (Audio|Components|Audio|Play (Variables|Default|GetAudio) 0.0))

(event Collision|EventActorBeginOverlap
  (params (OtherActor :type Actor%20Object%20Reference)))

(event EventTick
  (params (DeltaSeconds :type Float%20%28single-precision%29)))

(fn ConstructionScript)